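; BP_Enemy is an enemy that kills the player on contact and restarts the level.
; Overlap of its KillCollider with BP_Player toggles off the player's IM_NE input through the player controller and shows the WB_Died widget.
; It also fades out EnemyAudio and clears AIControllerClass, intended to remove the enemy AI.
; When the widget's FadeIn animation finishes, a bound event reopens the current level by name.
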(event `self.KillCollider.OnComponentBeginOverlap`
  (params (OverlappedComponent :type "PrimitiveComponent Object Reference") (OtherActor :type "Actor Object Reference") (OtherComp :type "PrimitiveComponent Object Reference") (OtherBodyIndex :type Integer) (bFromSweep :type Boolean) (SweepResult :type "HitResult Structure (by ref)"))
  (bind _asbp_player (cast `/Game/_Main/Player/BP_Player` OtherActor))
  (bind _bp_player_controller (`/Game/_Main/Player/BP_Player.BP Player Controller` _asbp_player))
  (`/Game/_Main/Player/BP_PlayerController.ToggleInput` _bp_player_controller false "/Game/_Main/Player/Inputs/IM_NE.IM_NE")
  (bind _returnvalue (`|CreateWidget` "/Game/_Main/UI/WB_Died.WB_Died_C" _bp_player_controller))
  (bind _output_get (set `self.WB_Died` _returnvalue))
  (`UserWidget.AddToViewport` _output_get 0)
  (`UserWidget.BindToAnimationFinished` _output_get (`/Game/_Main/UI/WB_Died.FadeIn` _output_get) (delegate `RestartLevel`))
  (`AudioComponent.FadeOut` (`self.EnemyAudio`) 0.5 0.0 "Linear")
  ;[1 1 1] Remove Enemy AI on Player killed
  (set `self.AIControllerClass` null))

(event `RestartLevel`
  (bind _returnvalue (`GameplayStatics.GetCurrentLevelName` true))
  (`GameplayStatics.OpenLevel` (`KismetStringLibrary.Conv_StringToName` _returnvalue)))

(fn `UserConstructionScript`)