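; LandMark_3 is a sound trigger actor for a landmark, built around an overlap Sphere.
; The first overlap passes a DoOnce, toggles the Landmark3 component's active state and spawns two actors, NewSound and NewSound2, at their stored locations.
; Later overlaps do nothing, and the construction script is empty.
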(event `self.Sphere.OnComponentBeginOverlap`
  (params (OverlappedComponent :type "PrimitiveComponent Object Reference") (OtherActor :type "Actor Object Reference") (OtherComp :type "PrimitiveComponent Object Reference") (OtherBodyIndex :type Integer) (bFromSweep :type Boolean) (SweepResult :type "HitResult Structure (by ref)"))
  (`/Engine/EditorBlueprintResources/StandardMacros.DoOnce` false
    (:`Completed`
      (`ActorComponent.ToggleActive` (`self.Landmark_3`))
      (`|SpawnActorFromClass` (`self.NewSound`) (`KismetMathLibrary.Conv_VectorToTransform` (`self.NewSoundLocation`)) "Undefined" "MultiplyWithRoot" null null)
      (`|SpawnActorFromClass` (`self.NewSound2`) (`KismetMathLibrary.Conv_VectorToTransform` (`self.NewSoundLocation2`)) "Undefined" "MultiplyWithRoot" null null))))

(fn `UserConstructionScript`)